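; BP_WorldManager controls the simulation's speed and reports population counts for a predator and prey world.
; Each tick it sets global time dilation from its TimeScale variable.
; It also gathers every BP_Prey and BP_Predator actor per tick and prints both counts on screen as a debug readout.
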(event EventBeginPlay)

(event Collision|EventActorBeginOverlap
  (params (OtherActor :type Actor%20Object%20Reference)))

(event EventTick
  (params (DeltaSeconds :type Float%20%28single-precision%29))
  ;[1 1 1] controls speed of the world
  (Utilities|Time|SetGlobalTimeDilation (Variables|Default|GetTimeScale))
  ;[1 1 1] Displays number of prey and predators in scene, i used it for debugging but leaving it in so you can track numbers easily
  (bind _outactors (Actor|GetAllActorsOfClass "/Game/BluePrints/ReAttempt/BP_Prey.BP_Prey_C"))
  (bind _output_get (Variables|Default|SetPreyString "Prey:     "))
  (Development|PrintString (Utilities|String|Append _output_get (Utilities|String|ToString(Integer) (Utilities|Array|Length _outactors))) true true "(R=0.000000,G=0.660000,B=1.000000,A=1.000000)" 0.0)
  (bind _outactors_2 (Actor|GetAllActorsOfClass "/Game/BluePrints/ReAttempt/BP_Predator.BP_Predator_C"))
  (bind _output_get_2 (Variables|Default|SetPredString "Predators:    "))
  (Development|PrintString (Utilities|String|Append _output_get_2 (Utilities|String|ToString(Integer) (Utilities|Array|Length _outactors_2))) true true "(R=0.000000,G=0.660000,B=1.000000,A=1.000000)" 0.0))

(fn ConstructionScript)