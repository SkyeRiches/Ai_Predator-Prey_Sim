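; AI controller for prey in a predator-prey life simulation, randomizing sex and heritable stats at spawn and running BT_Prey.
; Perception updates sort predators, bushes and ready opposite-sex prey into enemy, food and mate lists.
; Tick updates energy, hunger, age and cooldowns; blackboard flags signal sex, threats, flee readiness and mating to the tree.
; Die stops the tree and leaves a corpse for predators to eat.
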(event OnTargetPerceptionUpdated(AIPerception)
  (params (Actor :type Actor%20Object%20Reference) (Stimulus :type AI%20Stimulus%20Structure))
  (bind (_age _expirationage) (Utilities|Struct|BreakAIStimulus Stimulus))
  ;[1 1 1] Store items in view
  (if (>= _age _expirationage)
    (CallFunction|RemovePerceivedItem Actor)
    (else
      (CallFunction|AddNewPerceivedItem Actor)
      (Utilities|FlowControl|Delay 0.2)
      (AI|Components|Blackboard|SetValueasBool (AI|GetBlackboard 0) (Utilities|Name|MakeLiteralName "EnemySpotted") false) ; This resets the enemy spotted bool on the blackboard\nso that it doesnt end up in an infinite loop of bailing from\nthe wander behaviour.
    )))

(event EventBeginPlay
  ;[1 1 1] Intialise
  (CallFunction|RandomStats)
  (CallFunction|SetInitialValues)
  (AI|RunBehaviorTree "/Game/BluePrints/ReAttempt/BT_Prey.BT_Prey")
  (bind _asbp_prey_controller (Utilities|Casting|CastToBP_PreyController (AI|GetAIController self)))
  (AI|Components|Blackboard|SetValueasBool (AI|GetBlackboard _asbp_prey_controller) (Utilities|Name|MakeLiteralName "Female") (Variables|Default|GetisFemale)) ; Tell the blackboard if its female
)

(event EventTick
  (params (DeltaSeconds :type Float%20%28single-precision%29))
  ;[1 1 1] update the stats of the ai and keep the location of the controlle the same as the pawn (this helps debug)
  (CallFunction|UpdateStats) ; changes the stats over time making the ai need to do different things
  (Transformation|SetActorLocation (Transformation|GetActorLocation (Pawn|GetControlledPawn)) false false))

(fn ConstructionScript)

(fn TakeDamage
  (params (Damage :type Float%20%28double-precision%29))
  ;[1 1 1] Subtracts an amount from the hp of the ai
  (Variables|Default|SetHP (- (Variables|Default|GetHP) Damage)))

(fn MatingConsent
  (params (mating :type Boolean))
  ;[1 1 1] This starts the mating process. It sets it to be mating rather than ready to mate and changes a value on the blackboard to reflect this, which then unlocks a branch of the behaviour tree
  (bind _output_get (Variables|Default|SetisMating mating))
  (Variables|Default|SetReadyToMate false)
  (bind _asbp_prey_controller (Utilities|Casting|CastToBP_PreyController (AI|GetAIController self)))
  (AI|Components|Blackboard|SetValueasBool (AI|GetBlackboard _asbp_prey_controller) (Utilities|Name|MakeLiteralName "isMating") _output_get))

(fn SetInitialValues
  ;[1 1 1] Initialises all the start values for this ai
  (Variables|Default|SetHP (Variables|Default|GetMaxHP))
  (Variables|Default|SetEnergy (Variables|Default|GetMaxEnergy))
  (Variables|Default|SetCurrentMateCooldown (Variables|Default|GetMateCooldown))
  (bind _asbp_prey (Utilities|Casting|CastToBP_Prey (Pawn|GetControlledPawn self)))
  (Default|SetMoveSpeed _asbp_prey (Variables|Default|GetMoveSpeed)))

(fn RandomStats
  ;[1 1 1] Generates random values within ranges, for the core stats of the ai. These factors are the ones passed down in genetics, this is why its random, so not all ai end up inheriting the same values
  (Variables|Default|SetMaxEnergy (Math|Random|RandomFloatinRange 1e+02 1.2e+02))
  (Variables|Default|SetMateCooldown (Math|Random|RandomFloatinRange 1e+02 125.0))
  (Variables|Default|SetMaxHP (Math|Random|RandomFloatinRange 8e+01 1e+02))
  (Variables|Default|SetMaxAge (Math|Random|RandomFloatinRange 1.25e+03 1.5e+03))
  (Variables|Default|SetMoveSpeed (Math|Random|RandomFloatinRange 5e+02 6e+02))
  (Variables|Default|SetisFemale (Math|Random|RandomBool)))

(fn AddNewPerceivedItem
  (params (Object :type Actor%20Object%20Reference))
  (bind _isfemale (Variables|Default|GetisFemale))
  ;[1 1 1] if its predator, add it to list of enemies and tell the blackboard a new enemy has been spotted
  (bind _asbp_predator (Utilities|Casting|CastToBP_Predator Object)
    (:then
      (Utilities|Array|AddUnique (Variables|Default|GetEnemies) _asbp_predator)
      (AI|Components|Blackboard|SetValueasBool (AI|GetBlackboard self) (Utilities|Name|MakeLiteralName "EnemySpotted") true))
    (:CastFailed
      ;[1 1 1] If its a bush, add it to list of food
      (bind _asbp_food_bush (Utilities|Casting|CastToBP_FoodBush Object)
        (:then
          (Utilities|Array|AddUnique (Variables|Default|GetFood) _asbp_food_bush))
        (:CastFailed
          ;[1 1 1] If it is prey and ready to mate and opposite sex, add it to list of mates
          (bind _asbp_prey (Utilities|Casting|CastToBP_Prey Object))
          (bind _asbp_prey_controller (Utilities|Casting|CastToBP_PreyController (AI|GetAIController _asbp_prey)))
          (if (Variables|BP_PreyController_C|GetReadyToMate _asbp_prey_controller) ; if it is ready to mate
            (if (Variables|BP_PreyController_C|GetisFemale _asbp_prey_controller) ; if it is female
              (if (not _isfemale) ; if its female and this isnt,\nadd it to list
                (if (Utilities|IsValid _asbp_prey) :!label _label ; ensure the other object is valid before adding
                  (Utilities|Array|AddUnique (Variables|Default|GetMates) _asbp_prey)))
              (elif _isfemale ; if its not female and this is\nadd it to list
                (goto _label)))))))))

(fn RemovePerceivedItem
  (params (Object :type Actor%20Object%20Reference))
  ;[1 1 1] Remove predator from list of enemies
  (bind _asbp_predator (Utilities|Casting|CastToBP_Predator Object)
    (:then
      (Utilities|Array|RemoveItem (Variables|Default|GetEnemies) _asbp_predator))
    (:CastFailed
      ;[1 1 1] Remove bush from list of food
      (bind _asbp_food_bush (Utilities|Casting|CastToBP_FoodBush Object)
        (:then
          (Utilities|Array|RemoveItem (Variables|Default|GetFood) _asbp_food_bush))
        (:CastFailed
          ;[1 1 1] Remove fellow prey from list of mates
          (bind _asbp_prey (Utilities|Casting|CastToBP_Prey Object))
          (Utilities|Array|RemoveItem (Variables|Default|GetMates) _asbp_prey))))))

(fn UpdateStats
  (bind _returnvalue (AI|GetBlackboard 0))
  (bind _returnvalue_2 (Utilities|Name|MakeLiteralName "ReadyToFlee"))
  (if (or (Variables|Default|GetisSleeping) (Variables|Default|GetisMating)) ; if it is sleeping or mating, the stats for\nenergy and hunger shouldnt go down\notherwise they end up dying mid task
    _
    (else
      ;[1 1 1] Update Energy
      (Variables|Default|SetEnergy (- (Variables|Default|GetEnergy) (* (Utilities|Time|GetWorldDeltaSeconds) (Variables|Default|GetEnergyDrain))))
      ;[1 1 1] Update Hunger
      (Variables|Default|SetHunger (+ (Variables|Default|GetHunger) (* (Utilities|Time|GetWorldDeltaSeconds) (Variables|Default|GetHungerDrain))))))
  ;[1 1 1] Update Age
  (Variables|Default|SetAge (+ (Variables|Default|GetAge) (Utilities|Time|GetWorldDeltaSeconds)))
  ;[1 1 1] Update Mate Cooldown
  (if (not (or (Variables|Default|GetReadyToMate) (Variables|Default|GetisMating)))
    (Variables|Default|SetCurrentMateCooldown (- (Variables|Default|GetCurrentMateCooldown) (Utilities|Time|GetWorldDeltaSeconds)))
    ;[1 1 1] reduce flee cooldown value, if it reaches zero, tell blackboard it can now flee again
    (bind _output_get (Variables|Default|SetFleeCooldown (- (Variables|Default|GetFleeCooldown) (Utilities|Time|GetWorldDeltaSeconds))))
    (if (<= _output_get 0.0)
      (AI|Components|Blackboard|SetValueasBool _returnvalue _returnvalue_2 true)
      (Variables|Default|SetFleeCooldown 0.0) ; stop it from going into negatives
      (else
        (AI|Components|Blackboard|SetValueasBool _returnvalue _returnvalue_2 false)))))

(fn Die
  (AI|Logic|StopLogic (Variables|Default|GetBrainComponent self) "") ; Stops the behaviour tree from running
  (Game|SpawnActorfromClass "/Game/BluePrints/ReAttempt/BP_Corpse.BP_Corpse_C" (Transformation|GetActorTransform (Pawn|GetControlledPawn)) "Undefined" "MultiplyWithRoot" 0 0) ; spawn a corpse as this is what predators feed on
  ;[1 1 1] Destroy the pawn and then this object
  (Actor|DestroyActor (Pawn|GetControlledPawn))
  (Actor|DestroyActor))